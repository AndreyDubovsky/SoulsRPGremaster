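; Player hero character with camera-relative movement, sprinting, rolling and montage-based attacks, built for multiplayer.
; Sprint sets walk speed locally and on the server, with a replicated flag's OnRep messaging the AnimInstance.
; Roll and attack inputs go through server events that multicast montages, with completion reporting back to the server.
; Only light attack has a montage, CurrentlyAttacking is never set true, and the multicast roll ignores its State input.
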(event Custom|Server_ToggleSprint
  (params (State :type Boolean))
  ;[1 1 1] Sprint system
  (CallFunction|FSprintSwitch State))

(event Custom|Server_Rolling
  (params (Rolling :type Boolean))
  ;[1 1 1] Rolling System
  (if Rolling
    (Variables|Default|SetRolling true)
    (CallFunction|MultiRolling (Variables|Character|GetMesh) "/Game/_Main/Player/GreystoneRoll_Montage.GreystoneRoll_Montage" true)
    (else
      (Variables|Default|SetRolling false)
      (CallFunction|MultiRolling 0 "/Game/_Main/Player/GreystoneRoll_Montage.GreystoneRoll_Montage" false))))

(event Custom|Multi_Rolling
  (params (Mesh :type Skeletal%20Mesh%20Component%20Object%20Reference) (Montage :type Anim%20Montage%20Object%20Reference) (State :type Boolean))
  (bind _returnvalue (Components|SkeletalMesh|GetAnimInstance (Variables|Character|GetMesh)))
  ;[1 1 1] Rolling System
  (if true
    (Class|INTHeroAnimBP|RollingState(Message) _returnvalue true)
    (Animation|Montage|PlayMontage Mesh Montage
      (:OnCompleted
        (CallFunction|ServerRolling false)))
    (else
      (Class|INTHeroAnimBP|RollingState(Message) _returnvalue false))))

(event Custom|Server_TryToActivateAbility
  (params (Attacks :type E_PlayerAttackks%20Enum :default "NewEnumerator0"))
  (if (and (not (Variables|Attacking|GetCurrentlyAttacking)) (not (Variables|Default|GetRolling)))
    (switch Utilities|FlowControl|Switch|SwitchonE_PlayerAttackks Attacks
      (:NewEnumerator0
        (Variables|Attacking|SetCurrentlyAttacking false)
        (CallFunction|MultiPlayMontage (Variables|Character|GetMesh) "/Game/_Main/Player/LightAttack_Montage.LightAttack_Montage" "None")))))

(event Custom|Multi_PlayMontage
  (params (InSkeletalMeshComponent :type Skeletal%20Mesh%20Component%20Object%20Reference) (MontageToPlay :type Anim%20Montage%20Object%20Reference) (StartingSection :type Name))
  (Animation|Montage|PlayMontage InSkeletalMeshComponent MontageToPlay 1.0 0.0 StartingSection
    (:OnCompleted
      (CallFunction|ServerEndAttack))))

(event Custom|Server_EndAttack
  (Variables|Attacking|SetCurrentlyAttacking false))

(event Input|ActionEvents|InputActionSprint
  (params (Key :type Key%20Structure :default "None"))
  ;[1 1 1] Sprint system
  (:Pressed
    (CallFunction|FSprintSwitch true) ; If player press shift key TRUE
  )
  (:Released
    (CallFunction|FSprintSwitch false) ; If player press shift key False
  ))

(event Input|ActionEvents|InputActionRolling
  (params (Key :type Key%20Structure :default "None"))
  ;[1 1 1] Rolling System
  (:Pressed
    (if (not (Variables|Default|GetRolling))
      (CallFunction|ServerRolling true))))

(event Input|ActionEvents|InputActionPrimary
  (params (Key :type Key%20Structure :default "None"))
  (:Pressed
    (CallFunction|ServerTrytoActivateAbility "NewEnumerator0")))

(event Input|ActionEvents|InputActionSecondary
  (params (Key :type Key%20Structure :default "None"))
  (:Pressed
    (CallFunction|ServerTrytoActivateAbility "NewEnumerator1")))

(event Input|AxisEvents|InputAxisTurn
  (params (AxisValue :type Float%20%28single-precision%29))
  ;[1 1 1] Movement
  (Pawn|Input|AddControllerYawInput AxisValue))

(event Input|AxisEvents|InputAxisLookUp
  (params (AxisValue :type Float%20%28single-precision%29))
  ;[1 1 1] Movement
  (Pawn|Input|AddControllerPitchInput AxisValue))

(event Input|AxisEvents|InputAxisMoveForward
  (params (AxisValue :type Float%20%28single-precision%29))
  ;[1 1 1] Movement
  (Pawn|Input|AddMovementInput (Math|Vector|GetForwardVector (Math|Rotator|MakeRotator 0.0 0.0 (.Yaw (Math|Rotator|BreakRotator (Pawn|GetControlRotation :!class /Script/Engine.Pawn))))) AxisValue false))

(event Input|AxisEvents|InputAxisMoveRight
  (params (AxisValue :type Float%20%28single-precision%29))
  ;[1 1 1] Movement
  (Pawn|Input|AddMovementInput (Math|Vector|GetRightVector (Math|Rotator|MakeRotator 0.0 0.0 (.Yaw (Math|Rotator|BreakRotator (Pawn|GetControlRotation :!class /Script/Engine.Pawn))))) AxisValue false))

(fn ConstructionScript
  (|CallParentFunction))

(fn FSprintSwitch
  (params (SprintState :type Boolean))
  (bind _charactermovement (Variables|Character|GetCharacterMovement))
  (bind _charactermovement_2 (Variables|Character|GetCharacterMovement))
  (LocalVariables|SetLocalSprint SprintState)
  (Networking|SwitchHasAuthority
    (:Authority
      (if (LocalVariables|GetLocalSprint)
        (Variables|/Script/Engine.CharacterMovementComponent|SetMaxWalkSpeed _charactermovement (Variables|Default|GetSprintSpeed))
        (Variables|Default|SetSprinting true)
        (else
          (Variables|/Script/Engine.CharacterMovementComponent|SetMaxWalkSpeed _charactermovement (Variables|Default|GetJogSpeed))
          (Variables|Default|SetSprinting false))))
    (:Remote
      (CallFunction|ServerToggleSprint (LocalVariables|GetLocalSprint))
      (if (LocalVariables|GetLocalSprint)
        (Variables|/Script/Engine.CharacterMovementComponent|SetMaxWalkSpeed _charactermovement_2 (Variables|Default|GetSprintSpeed))
        (else
          (Variables|/Script/Engine.CharacterMovementComponent|SetMaxWalkSpeed _charactermovement_2 (Variables|Default|GetJogSpeed))))))
  (return))

(fn OnRepSprinting
  (bind _mesh (Variables|Character|GetMesh))
  (bind _returnvalue (Components|SkeletalMesh|GetAnimInstance _mesh))
  (if (Variables|Default|GetSprinting)
    (Class|INTHeroAnimBP|SprintState(Message) _returnvalue true)
    (else
      (Class|INTHeroAnimBP|SprintState(Message) _returnvalue false))))